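; BP_Tree is a tree actor that grows in random, timed steps after BeginPlay.
; A DoN node with a random limit drives a loop that waits a few seconds, then calls Grow to add a random amount to the mesh's relative scale.
; The loop repeats through DoN unless its value equals zero, in which case it enables query and physics collision and prints a message.
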(event `self.ReceiveBeginPlay`
  (bind _counter (`/Engine/EditorBlueprintResources/StandardMacros.Do N` (`KismetMathLibrary.RandomIntegerInRange` 1 5) :!label _label)
    (:`Exit`
      (`KismetSystemLibrary.Delay` (`KismetMathLibrary.RandomFloatInRange` 3.0 5.0))
      (`self.Grow`)
      (if (== _counter 0)
        (`PrimitiveComponent.SetCollisionEnabled` (`self.SM_Generic_Tree_03`) "QueryAndPhysics")
        (`KismetSystemLibrary.PrintText` "Collision Enabled")
        (else
          (goto _label))))))

(event `Grow`
  (bind _sm_generic_tree_03 (`self.SM_Generic_Tree_03`))
  (`SceneComponent.SetRelativeScale3D` _sm_generic_tree_03 (+ (`SceneComponent.RelativeScale3D` _sm_generic_tree_03) (`KismetMathLibrary.RandomFloatInRange` 0.2 0.4))))

(fn `UserConstructionScript`)